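; BP_Hamburger is a tappable burger that calls RenewPoop on the player when touched or clicked, then destroys itself.
; On a first-time save, BeginPlay waits briefly, pauses the game and plays a guide sound.
; A mesh hit triggers delayed removal without the renewal.
; Both removal paths share cleanup that, on first time, clears the flag, stops the sound, unpauses and saves through MainGameInstance.
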(event `self.ReceiveBeginPlay`
  (bind _asmain_game_instance (cast `MainGameInstance` (`GameplayStatics.GetGameInstance`)))
  (if (`DataSaver.Is_First_Time` (`MainGameInstance.ASaveObj` _asmain_game_instance))
    (`KismetSystemLibrary.Delay` 2.5)
    (`GameplayStatics.SetGamePaused` true)
    (bind _returnvalue (`GameplayStatics.SpawnSound2D` "/Game/Sound/GuideBurger.GuideBurger" 1.0 1.0 0.0 null false false))
    (set `self.SomeAudio` _returnvalue)))

(event `self.hamburger.OnComponentHit`
  (params (HitComponent :type "PrimitiveComponent Object Reference") (OtherActor :type "Actor Object Reference") (OtherComp :type "PrimitiveComponent Object Reference") (NormalImpulse :type "Vector Structure") (Hit :type "HitResult Structure (by ref)"))
  (`KismetSystemLibrary.Delay` 5.0)
  (bind _asmain_game_instance (cast `MainGameInstance` (`GameplayStatics.GetGameInstance`) :!label _label))
  (bind _asaveobj (`MainGameInstance.ASaveObj` _asmain_game_instance))
  (if (`DataSaver.Is_First_Time` _asaveobj)
    (set `DataSaver.Is_First_Time` false _asaveobj)
    (`ActorComponent.SetActive` (`self.SomeAudio`) false false)
    (`GameplayStatics.SetGamePaused` false)
    (`MainGameInstance.SaveGame` _asmain_game_instance))
  (`self.K2_DestroyActor`))

(event `self.Sphere.OnInputTouchBegin`
  (params (FingerIndex :type "ETouchIndex Enum" :default "Touch1") (TouchedComponent :type "PrimitiveComponent Object Reference"))
  (bind _asmain_player (cast `MainPlayer` (`GameplayStatics.GetPlayerPawn` 0) :!label _label_2))
  (`MainPlayer.renew_poop` _asmain_player)
  (goto _label))

(event `self.Sphere.OnClicked`
  (params (TouchedComponent :type "PrimitiveComponent Object Reference") (ButtonPressed :type "Key Structure"))
  (goto _label_2))

(fn `UserConstructionScript`)